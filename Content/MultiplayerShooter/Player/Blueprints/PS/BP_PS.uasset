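; Player state for the multiplayer shooter that holds a player's named stats and handles the end-of-game screen on the client.
; A server event turns an add or subtract request into a signed value, then multicasts it to the matching stat object in the PlayerInfo map.
; A getter reads a stat's current value by name.
; StopGame clears all widgets, shows the leaderboard and sets the pause state.
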(event `CLIENT:StopGame`
  (params (bPaused :type Boolean))
  (`WidgetLayoutLibrary.RemoveAllWidgets`)
  (bind _returnvalue (`|CreateWidget` "/Game/MultiplayerShooter/Player/Widgets/Liderboard/WBP_Liderboard.WBP_Liderboard_C"))
  (`UserWidget.AddToViewport` _returnvalue 10)
  (`GameplayStatics.SetGamePaused` bPaused))

(event `SERVER:ChangePlayerInfo`
  (params (NameStat :type "String (by ref)") (MathDoing :type "/Game/MultiplayerShooter/Player/Blueprints/Components/Data/E_TypeMathDoing Enum" :default "NewEnumerator0") (Value :type "Float (double-precision)"))
  (`self.ChangePlayerInfo` NameStat MathDoing Value))

(event `MULTICAST:ChangePlayerInfoInObject`
  (params (Value :type "Float (double-precision)") (NameStat :type String))
  (bind _basestat (message `/Game/MultiplayerShooter/Player/Blueprints/Components/StatsSystem/BPI_Stat.GetBaseStat` (`BlueprintMapLibrary.Map_Find` (`self.PlayerInfo`) NameStat)))
  (`/Game/MultiplayerShooter/Player/Blueprints/Components/StatsSystem/BP_BaseStat.ChangeStat` _basestat Value))

(fn `ChangePlayerInfo`
  (params (NameStat :type "String (by ref)") (MathDoing :type "/Game/MultiplayerShooter/Player/Blueprints/Components/Data/E_TypeMathDoing Enum" :default "NewEnumerator0") (Value :type "Float (double-precision)"))
  (locals (L_StatData :type "/Game/MultiplayerShooter/Player/Blueprints/Components/Data/S_Stat Structure") (L_Value :type "Float (double-precision)") (L_BaseStat :type "/Game/MultiplayerShooter/Player/Blueprints/Components/StatsSystem/BP_BaseStat Object Reference"))
  (set `local.L_Value` (`KismetMathLibrary.Abs` Value))
  (switch `/Game/MultiplayerShooter/Player/Blueprints/Components/Data/E_TypeMathDoing` (`local.MathDoing`)
    (:`NewEnumerator0`
      _)
    (:`NewEnumerator1`
      (set `local.L_Value` (* (`local.L_Value`) -1.0))))
  (`self.MULTICAST:ChangePlayerInfoInObject` (`local.L_Value`) (`local.NameStat`)))

(fn `GetDataFromPlayerInfo`
  (params (NameInfo :type String))
  (returns (CurrentValue :type "Float (double-precision)"))
  (bind _basestat (message `/Game/MultiplayerShooter/Player/Blueprints/Components/StatsSystem/BPI_Stat.GetBaseStat` (`BlueprintMapLibrary.Map_Find` (`self.PlayerInfo`) NameInfo)))
  (return (`/Game/MultiplayerShooter/Player/Blueprints/Components/StatsSystem/BP_BaseStat.CurrentValue` _basestat)))

(fn `GetPS`
  (returns (PS :type "/Game/MultiplayerShooter/Player/Blueprints/PS/BP_PS Object Reference"))
  (return self))

(fn `UserConstructionScript`)