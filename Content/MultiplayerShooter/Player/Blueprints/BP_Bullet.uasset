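; BP_Bullet is a projectile actor for a multiplayer shooter that damages what it hits and plays an impact effect.
; Its Box component's hit event passes the hit location and actor to HandlerCollision.
; Targets with a skeletal mesh component receive damage credited to the owner's instigator controller and a hit Niagara effect, while others get a generic impact effect.
; The bullet destroys itself after any hit.
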(event `self.Box.OnComponentHit`
  (params (HitComponent :type "PrimitiveComponent Object Reference") (OtherActor :type "Actor Object Reference") (OtherComp :type "PrimitiveComponent Object Reference") (NormalImpulse :type "Vector Structure") (Hit :type "HitResult Structure (by ref)"))
  (`self.HandlerCollision` Hit_Location OtherActor))

(fn `GetBullet`
  (returns (Bullet :type "/Game/MultiplayerShooter/Player/Blueprints/BP_Bullet Object Reference"))
  (return self))

(fn `HandlerCollision`
  (params (LocHit :type "Vector Structure") (ActorHited :type "Actor Object Reference"))
  (locals (L_FX :type "NiagaraSystem Object Reference"))
  (`/Engine/EditorBlueprintResources/StandardMacros.IsValid` (`self.GetComponentByClass` ActorHited "/Script/Engine.SkeletalMeshComponent")
    (:`Is Valid`
      (set `local.L_FX` "/Game/MultiplayerShooter/VFX/sA_Megapack_v1/sA_StylizedAttacksPack/FX/NiagaraSystems/NS_BasicHit_2.NS_BasicHit_2")
      (`GameplayStatics.ApplyDamage` (`local.ActorHited`) (`self.Damage`) (`self.GetInstigatorController` (`self.GetOwner`))))
    (:`Is Not Valid`
      (set `local.L_FX` "/Game/MultiplayerShooter/VFX/sA_Megapack_v1/sA_ShootingVfxPack/FX/NiagaraSystems/NS_Impact_1.NS_Impact_1")))
  (`NiagaraFunctionLibrary.SpawnSystemAtLocation` (`local.L_FX`) (`local.LocHit`))
  (`self.K2_DestroyActor`))

(fn `UserConstructionScript`)