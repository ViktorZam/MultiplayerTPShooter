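; Player weapon component for a multiplayer shooter, handling firing, reloading, weapon switching and per-type ammo with HUD updates.
; Data table rows supply each weapon's fire delay, sound and mesh, with the mesh swapped on a montage notify.
; Firing is timer-gated and aims muzzle-spawned bullets at a camera trace hit.
; Server-to-multicast RPCs relay shots, sounds and montages, with bullet spawning and post-reload ammo refills ending in client RPCs.
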(event `self.ReceiveBeginPlay`
  (`parent.ReceiveBeginPlay`)
  (bind _returnvalue (`|GetDataTableRow` "/Game/MultiplayerShooter/Player/Blueprints/Components/Data/DT_Weapon.DT_Weapon" (`KismetStringLibrary.Conv_StringToName` (`|GetEnumeratorNameAsString` (`self.CurrentTypeWeapon`))))
    (:`then`
      (set `self.CurrentWeaponData` _returnvalue))))

(event `ShootingHandler`
  (bind (_currentweapondata_mesh _currentweapondata_shootdelay) (break `/Game/MultiplayerShooter/Player/Blueprints/Components/Data/S_Weapon` (`self.CurrentWeaponData`)))
  ;[0.01042 0.01042 0.01042] Shooting
  (`/Engine/EditorBlueprintResources/StandardMacros.DoOnce` false :!label _label
    (:`Completed`
      (bind _noammo_ (`self.Fire`))
      (if (not _noammo_)
        (`self.SERVER:RecoilWeapon`))
      (`KismetSystemLibrary.K2_SetTimerDelegate` (`|CreateDelegate` :!event `StartResetShoot`) _currentweapondata_shootdelay))))

(event `ResetShoot`
  ;[0.01042 0.01042 0.01042] Shooting
  (goto _label :!via `Reset`))

(event `SERVER:SoundShoot`
  (params (Location :type "Vector Structure"))
  ;[0.01042 0.01042 0.01042] Shooting
  (`self.MULTICAST:SoundShoot` Location))

(event `MULTICAST:SoundShoot`
  (params (Location :type "Vector Structure"))
  (bind (_currentweapondata_mesh _currentweapondata_shootdelay _currentweapondata_soundshoot) (break `/Game/MultiplayerShooter/Player/Blueprints/Components/Data/S_Weapon` (`self.CurrentWeaponData`)))
  ;[0.01042 0.01042 0.01042] Shooting
  (`GameplayStatics.PlaySoundAtLocation` _currentweapondata_soundshoot Location (struct) 1.0 1.0 0.0 null null null null))

(event `SERVER:RecoilWeapon`
  ;[0.01042 0.01042 0.01042] Shooting
  (`self.MULTICAST:RecoilWeapon`))

(event `MULTICAST:RecoilWeapon`
  ;[0.01042 0.01042 0.01042] Shooting
  (`|PlayMontage` (`Character.Mesh` (`self.PlayerChar`)) "/Game/MultiplayerShooter/Player/Characters/Mannequins/Animations/Manny/AM_Fire_Rifle_Ironsights.AM_Fire_Rifle_Ironsights"))

(event `Multicast:SpawnBullet`
  (params (SpawnTransform :type "Transform Structure"))
  ;[0.01042 0.01042 0.01042] Shooting
  (`self.CLIENT:SpawnBullet` SpawnTransform))

(event `CLIENT:SpawnBullet`
  (params (SpawnTransform :type "Transform Structure"))
  (bind _playerchar (`self.PlayerChar`))
  ;[0.01042 0.01042 0.01042] Shooting
  (`|SpawnActorFromClass` "/Game/MultiplayerShooter/Player/Blueprints/BP_Bullet.BP_Bullet_C" SpawnTransform "AlwaysSpawn" "MultiplyWithRoot" _playerchar _playerchar))

(event `SERVER:SpawnBullet`
  (params (SpawnTransform :type "Transform Structure"))
  ;[0.01042 0.01042 0.01042] Shooting
  (`self.Multicast:SpawnBullet` SpawnTransform))

(event `ChangeWeapon`
  (params (TypeWeaponEquip :type "/Game/MultiplayerShooter/Player/Blueprints/Components/Data/E_TypeWeapon Enum" :default "NewEnumerator0"))
  ;[0.01042 0.01042 0.01042] Change weapon
  (`self.SERVER:SetCurrentTypeWeapon` TypeWeaponEquip)
  (set `self.StateChar` "NewEnumerator1")
  (`self.UpdateAmmoWidget`)
  (`self.ChangeWeaponOnSERVER`))

(event `SERVER:SetCurrentTypeWeapon`
  (params (CurrentTypeWeapon :type "/Game/MultiplayerShooter/Player/Blueprints/Components/Data/E_TypeWeapon Enum" :default "NewEnumerator0"))
  ;[0.01042 0.01042 0.01042] Change weapon
  (set `self.CurrentTypeWeapon` CurrentTypeWeapon))

(event `PlayMontageMULTICAST`
  ;[0.01042 0.01042 0.01042] Change weapon
  (bind _notifyname (`|PlayMontage` (`Character.Mesh` (`self.PlayerChar`)) "/Game/MultiplayerShooter/Player/Characters/Mannequins/Animations/Manny/AM_Equip_Rifle_Standing.AM_Equip_Rifle_Standing")
    (:`OnCompleted`
      (set `self.StateChar` "NewEnumerator0"))
    (:`OnNotifyBegin`
      (if (== _notifyname "ChangeWeapon")
        (bind _returnvalue (`|GetDataTableRow` "/Game/MultiplayerShooter/Player/Blueprints/Components/Data/DT_Weapon.DT_Weapon" (`KismetStringLibrary.Conv_StringToName` (`|GetEnumeratorNameAsString` (`self.CurrentTypeWeapon`))))
          (:`then`
            (bind _output_get (set `self.CurrentWeaponData` _returnvalue))
            (`StaticMeshComponent.SetStaticMesh` (`/Game/MultiplayerShooter/Player/Blueprints/BP_ThirdPersonCharacter.GunStaticMesh` (`self.PlayerChar`)) (break `/Game/MultiplayerShooter/Player/Blueprints/Components/Data/S_Weapon` _output_get))))))))

(event `ChangeWeaponOnSERVER`
  ;[0.01042 0.01042 0.01042] Change weapon
  (`self.PlayMontageMULTICAST`))

(event `Reload`
  (bind (_cachedataammocurrentweapon_currentinmagazineammo _cachedataammocurrentweapon_countammofitinmagazine _cachedataammocurrentweapon_inselfammo) (break `/Game/MultiplayerShooter/Player/Blueprints/Components/Data/S_Ammo` (`self.CacheDataAmmoCurrentWeapon`)))
  ;[0.01042 0.01042 0.01042] Change weapon
  (set `self.CacheDataAmmoCurrentWeapon` (`BlueprintMapLibrary.Map_Find` (`self.Ammo`) (`self.CurrentTypeWeapon`)))
  (if (> _cachedataammocurrentweapon_inselfammo 0)
    (if (!= _cachedataammocurrentweapon_currentinmagazineammo _cachedataammocurrentweapon_countammofitinmagazine)
      (set `self.StateChar` "NewEnumerator2")
      (`self.SERVER:Reload`))))

(event `CLIENT:UpdateAmmo`
  (bind (_cachedataammocurrentweapon_currentinmagazineammo _cachedataammocurrentweapon_countammofitinmagazine _cachedataammocurrentweapon_inselfammo) (break `/Game/MultiplayerShooter/Player/Blueprints/Components/Data/S_Ammo` (`self.CacheDataAmmoCurrentWeapon`)))
  (bind (_cachedataammocurrentweapon_currentinmagazineammo_2 _cachedataammocurrentweapon_countammofitinmagazine_2) (break `/Game/MultiplayerShooter/Player/Blueprints/Components/Data/S_Ammo` (`self.CacheDataAmmoCurrentWeapon`)))
  (bind _returnvalue (- _cachedataammocurrentweapon_countammofitinmagazine _cachedataammocurrentweapon_currentinmagazineammo))
  ;[0.01042 0.01042 0.01042] Change weapon
  (if (>= _returnvalue _cachedataammocurrentweapon_inselfammo)
    (bind _structout (setmembers `/Game/MultiplayerShooter/Player/Blueprints/Components/Data/S_Ammo` :`StructRef` (`self.CacheDataAmmoCurrentWeapon`) :`CurrentInMagazineAmmo` (+ _cachedataammocurrentweapon_currentinmagazineammo _cachedataammocurrentweapon_inselfammo) :`InSelfAmmo` 0))
    (`BlueprintMapLibrary.Map_Add` (`self.Ammo`) (`self.CurrentTypeWeapon`) _structout)
    (else
      (bind _structout_2 (setmembers `/Game/MultiplayerShooter/Player/Blueprints/Components/Data/S_Ammo` :`StructRef` (`self.CacheDataAmmoCurrentWeapon`) :`CurrentInMagazineAmmo` _cachedataammocurrentweapon_countammofitinmagazine_2 :`InSelfAmmo` (- _cachedataammocurrentweapon_inselfammo _returnvalue)))
      (`BlueprintMapLibrary.Map_Add` (`self.Ammo`) (`self.CurrentTypeWeapon`) _structout_2)))
  (`self.UpdateAmmoWidget`)
  (set `self.StateChar` "NewEnumerator0"))

(event `SERVER:Reload`
  ;[0.01042 0.01042 0.01042] Change weapon
  (`self.MULTICAST:Reload`))

(event `MULTICAST:Reload`
  ;[0.01042 0.01042 0.01042] Change weapon
  (`|PlayMontage` (`Character.Mesh` (`self.PlayerChar`)) "/Game/MultiplayerShooter/Player/Characters/Mannequins/Animations/Manny/AM_Reload_Rifle_Hip.AM_Reload_Rifle_Hip"
    (:`OnCompleted`
      (`self.CLIENT:UpdateAmmo`))))

(fn `CalculateSpawnBullet`
  (returns (BulletTransform :type "Transform Structure"))
  (locals (L_MuzzleSocLoc :type "Vector Structure") (L_BulletSpawnT :type "Transform Structure"))
  (bind _returnvalue (`SceneComponent.K2_GetComponentLocation` (`/Game/MultiplayerShooter/Player/Blueprints/BP_ThirdPersonCharacter.FollowCamera` (`self.PlayerChar`))))
  (bind _returnvalue_2 (+ _returnvalue (* (`SceneComponent.GetForwardVector` (`/Game/MultiplayerShooter/Player/Blueprints/BP_ThirdPersonCharacter.FollowCamera` (`self.PlayerChar`))) 10000.0)))
  (set `local.L_MuzzleSocLoc` (`SceneComponent.GetSocketLocation` (`/Game/MultiplayerShooter/Player/Blueprints/BP_ThirdPersonCharacter.GunStaticMesh` (`self.PlayerChar`)) "MuzzleSocket"))
  (bind (_outhit _returnvalue_3) (`KismetSystemLibrary.LineTraceSingleForObjects` _returnvalue _returnvalue_2 (`|MakeArray` "ObjectTypeQuery1" "ObjectTypeQuery2" "ObjectTypeQuery4" :!type "EObjectTypeQuery Enum")))
  (if _returnvalue_3
    (set `local.L_BulletSpawnT` (`KismetMathLibrary.MakeTransform` (`local.L_MuzzleSocLoc`) (`KismetMathLibrary.FindLookAtRotation` (`local.L_MuzzleSocLoc`) (`.ImpactPoint` (`GameplayStatics.BreakHitResult` _outhit)))))
    (else
      (set `local.L_BulletSpawnT` (`KismetMathLibrary.MakeTransform` (`local.L_MuzzleSocLoc`) (`KismetMathLibrary.FindLookAtRotation` (`local.L_MuzzleSocLoc`) _returnvalue_2)))))
  (`self.SERVER:SpawnBullet` (`local.L_BulletSpawnT`))
  (return (`local.L_BulletSpawnT`)))

(fn `Fire`
  (returns (`NoAmmo?` :type Boolean))
  (locals (L_MuzzleSocLoc :type "Vector Structure" :default (0.0 0.0 0.0)) (L_BulletSpawnT :type "Transform Structure") (L_AmmoData :type "/Game/MultiplayerShooter/Player/Blueprints/Components/Data/S_Ammo Structure"))
  (bind (_l_ammodata_currentinmagazineammo _l_ammodata_countammofitinmagazine _l_ammodata_inselfammo) (break `/Game/MultiplayerShooter/Player/Blueprints/Components/Data/S_Ammo` (`local.L_AmmoData`)))
  (bind _l_bulletspawnt_location (`KismetMathLibrary.BreakTransform` (`local.L_BulletSpawnT`)))
  (bind _output_get (set `local.L_AmmoData` (`BlueprintMapLibrary.Map_Find` (`self.Ammo`) (`self.CurrentTypeWeapon`))))
  (if (<= (`.CurrentInMagazineAmmo_14_8B29CF054E6C71855528658CC4BAA8C1` (break `/Game/MultiplayerShooter/Player/Blueprints/Components/Data/S_Ammo` _output_get)) 0)
    (`GameplayStatics.PlaySound2D` "/Game/MultiplayerShooter/Audio/Sounds/Weapons/MSS_NoAmmo.MSS_NoAmmo" 1.0 1.0 0.0 null null)
    (return true)
    (else
      (bind _bullettransform (`self.CalculateSpawnBullet`))
      (set `local.L_BulletSpawnT` _bullettransform)
      (bind _structout (setmembers `/Game/MultiplayerShooter/Player/Blueprints/Components/Data/S_Ammo` :`StructRef` (`local.L_AmmoData`) :`CurrentInMagazineAmmo` (- (`.CurrentInMagazineAmmo_14_8B29CF054E6C71855528658CC4BAA8C1` (break `/Game/MultiplayerShooter/Player/Blueprints/Components/Data/S_Ammo` (`local.L_AmmoData`))) 1)))
      (`BlueprintMapLibrary.Map_Add` (`self.Ammo`) (`self.CurrentTypeWeapon`) _structout)
      (bind _foundwidgets (`WidgetBlueprintLibrary.GetAllWidgetsOfClass` "/Game/MultiplayerShooter/Player/Widgets/WBP_PlayerHUD.WBP_PlayerHUD_C"))
      (`WCPP_PlayerHUD.UpdateAmmoWidgetComponent` (`|GetArrayItem` _foundwidgets) _l_ammodata_currentinmagazineammo _l_ammodata_inselfammo)
      (`self.SERVER:SoundShoot` _l_bulletspawnt_location)
      (return false))))

(fn `StartResetShoot`
  (`self.ResetShoot`))

(fn `UpdateAmmoWidget`
  (bind (_cachedataammocurrentweapon_currentinmagazineammo _cachedataammocurrentweapon_countammofitinmagazine _cachedataammocurrentweapon_inselfammo) (break `/Game/MultiplayerShooter/Player/Blueprints/Components/Data/S_Ammo` (`self.CacheDataAmmoCurrentWeapon`)))
  (set `self.CacheDataAmmoCurrentWeapon` (`BlueprintMapLibrary.Map_Find` (`self.Ammo`) (`self.CurrentTypeWeapon`)))
  (bind _foundwidgets (`WidgetBlueprintLibrary.GetAllWidgetsOfClass` "/Game/MultiplayerShooter/Player/Widgets/WBP_PlayerHUD.WBP_PlayerHUD_C"))
  (`WCPP_PlayerHUD.UpdateAmmoWidgetComponent` (`|GetArrayItem` _foundwidgets) _cachedataammocurrentweapon_currentinmagazineammo _cachedataammocurrentweapon_inselfammo))