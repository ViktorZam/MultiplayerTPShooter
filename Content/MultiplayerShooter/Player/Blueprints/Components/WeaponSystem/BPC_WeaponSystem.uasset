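; Player weapon component for a multiplayer shooter, handling firing, recoil, weapon switching, reloading and per-type ammo with HUD updates.
; Firing traces from the camera to aim bullets from the muzzle, relaying spawn and sound through server and multicast RPCs.
; Camera shake and random kick add recoil, with timer-driven interpolation for anim recoil decay and aim stabilization.
; DT_Weapon rows supply weapon data, and equip and reload montages drive swaps and ammo refills.
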(event `self.ReceiveBeginPlay`
  (`parent.ReceiveBeginPlay`)
  (`self.Update Info Weapon`))

(event `ShootingHandler`
  (bind (_currentweapondata_mesh _currentweapondata_shootdelay) (break `/Game/MultiplayerShooter/Player/Blueprints/Components/WeaponSystem/Data/S_Weapon` (`self.CurrentWeaponData`)))
  ;[0.01042 0.01042 0.01042] Shooting
  (`/Engine/EditorBlueprintResources/StandardMacros.DoOnce` false :!label _label
    (:`Completed`
      (bind _noammo_ (`self.Fire`))
      (bind _output_get (set `self.No Ammo?` _noammo_))
      (if (not _output_get)
        (`self.SERVER:RecoilAnimWeapon`)
        (`self.CLIENT:CalculateRecoilController`))
      (`KismetSystemLibrary.K2_SetTimerDelegate` (`|CreateDelegate` :!event `StartResetShoot`) _currentweapondata_shootdelay))))

(event `ResetShoot`
  ;[0.01042 0.01042 0.01042] Shooting
  (goto _label :!via `Reset`))

(event `MULTICAST:RecoilAnimWeapon`
  ;[0.01042 0.01042 0.01042] Shooting
  ;;[0 0 0] Recoil
  (bind _animbp (message `/Game/MultiplayerShooter/Player/Characters/Mannequins/Animations/BPI/BPI_AnimBP.GetMannyAnimBP` (`SkeletalMeshComponent.GetAnimInstance` (`Character.Mesh` (`self.PlayerChar`)))))
  (set `self.AlphaAnimRecoilWeapon` (`KismetMathLibrary.FClamp` (+ (`/Game/MultiplayerShooter/Player/Characters/Mannequins/Animations/ABP_Manny.AlphaRecoilFire` _animbp) 0.5)))
  (`self.CLIENT:LoweringRecoil`))

(event `SERVER:RecoilAnimWeapon`
  ;[0.01042 0.01042 0.01042] Shooting
  ;;[0 0 0] Recoil
  (`self.MULTICAST:RecoilAnimWeapon`))

(event `SERVER:SoundShoot`
  (params (Location :type "Vector Structure"))
  ;[0.01042 0.01042 0.01042] Shooting
  (`self.MULTICAST:SoundShoot` Location))

(event `CLIENT:LoweringRecoil`
  ;[0.01042 0.01042 0.01042] Shooting
  ;;[0 0 0] Recoil
  (`/Engine/EditorBlueprintResources/StandardMacros.DoOnce` false :!label _label_2
    (:`Completed`
      (`KismetSystemLibrary.K2_SetTimerDelegate` (`|CreateDelegate` :!event `LoweringAnimRecoil`) 0.016 true))))

(event `MULTICAST:SoundShoot`
  (params (Location :type "Vector Structure"))
  (bind (_currentweapondata_mesh _currentweapondata_shootdelay _currentweapondata_soundshoot) (break `/Game/MultiplayerShooter/Player/Blueprints/Components/WeaponSystem/Data/S_Weapon` (`self.CurrentWeaponData`)))
  ;[0.01042 0.01042 0.01042] Shooting
  (`GameplayStatics.PlaySoundAtLocation` _currentweapondata_soundshoot Location (struct) 1.0 1.0 0.0 null null null null))

(event `ResetTimerLoweringRecoil`
  ;[0.01042 0.01042 0.01042] Shooting
  ;;[0 0 0] Recoil
  (goto _label_2 :!via `Reset`))

(event `CLIENT:CalculateRecoilController`
  ;[0.01042 0.01042 0.01042] Shooting
  ;;[0 0 0] Recoil
  (bind _pc (message `/Game/MultiplayerShooter/Player/Blueprints/BPI/BPI_PC.GetPC` (`Pawn.GetController` (`self.PlayerChar`))))
  (`PlayerCameraManager.StartCameraShake` :`self` (`PlayerController.PlayerCameraManager` _pc) :`ShakeClass` "/Game/MultiplayerShooter/Player/Blueprints/Components/WeaponSystem/BP_ShootingShake.BP_ShootingShake_C")
  (bind _foundwidgets (`WidgetBlueprintLibrary.GetAllWidgetsOfClass` "/Game/MultiplayerShooter/Player/Widgets/WBP_PlayerHUD.WBP_PlayerHUD_C"))
  (`WCPP_PlayerHUD.UpdateCrosshairAfterShoot` (`|GetArrayItem` _foundwidgets))
  (`self.CalculateRecoilController`))

(event `Multicast:SpawnBullet`
  (params (SpawnTransform :type "Transform Structure"))
  ;[0.01042 0.01042 0.01042] Shooting
  (`self.CLIENT:SpawnBullet` SpawnTransform))

(event `SERVER:SetLoweringRecoil`
  (params (`Alpha Recoil Fire Rifle` :type "Float (single-precision)"))
  ;[0.01042 0.01042 0.01042] Shooting
  ;;[0 0 0] Recoil
  (`self.MULTICAST:SetLoweringRecoil` `Alpha Recoil Fire Rifle`))

(event `CLIENT:SpawnBullet`
  (params (SpawnTransform :type "Transform Structure"))
  (bind _playerchar (`self.PlayerChar`))
  ;[0.01042 0.01042 0.01042] Shooting
  (`|SpawnActorFromClass` "/Game/MultiplayerShooter/Player/Blueprints/BP_Bullet.BP_Bullet_C" SpawnTransform "AlwaysSpawn" "MultiplyWithRoot" _playerchar _playerchar))

(event `SERVER:SpawnBullet`
  (params (SpawnTransform :type "Transform Structure"))
  ;[0.01042 0.01042 0.01042] Shooting
  (`self.Multicast:SpawnBullet` SpawnTransform))

(event `MULTICAST:SetLoweringRecoil`
  (params (AlphaAnimRecoilWeapon :type "Float (single-precision)"))
  ;[0.01042 0.01042 0.01042] Shooting
  ;;[0 0 0] Recoil
  (set `self.AlphaAnimRecoilWeapon` AlphaAnimRecoilWeapon))

(event `ChangeWeapon`
  (params (TypeWeaponEquip :type "/Game/MultiplayerShooter/Player/Blueprints/Components/WeaponSystem/Data/E_TypeWeapon Enum" :default "NewEnumerator0"))
  ;[0.01042 0.01042 0.01042] Change weapon
  (`self.SERVER:SetCurrentTypeWeapon` TypeWeaponEquip)
  (set `self.StateChar` "NewEnumerator1")
  (`self.UpdateAmmoWidget`)
  (`self.ChangeWeaponOnSERVER`))

(event `SERVER:SetCurrentTypeWeapon`
  (params (CurrentTypeWeapon :type "/Game/MultiplayerShooter/Player/Blueprints/Components/WeaponSystem/Data/E_TypeWeapon Enum" :default "NewEnumerator0"))
  ;[0.01042 0.01042 0.01042] Change weapon
  (bind _output_get (set `self.CurrentTypeWeapon` CurrentTypeWeapon))
  (bind _animbp (message `/Game/MultiplayerShooter/Player/Characters/Mannequins/Animations/BPI/BPI_AnimBP.GetMannyAnimBP` (`SkeletalMeshComponent.GetAnimInstance` (`Character.Mesh` (`self.PlayerChar`)))))
  (set `/Game/MultiplayerShooter/Player/Characters/Mannequins/Animations/ABP_Manny.TypeWeapon` _output_get _animbp))

(event `ChangeWeaponOnSERVER`
  ;[0.01042 0.01042 0.01042] Change weapon
  (`self.MULTICAST:ChangeWeapon`))

(event `MULTICAST:ChangeWeapon`
  ;[0.01042 0.01042 0.01042] Change weapon
  (bind _notifyname (`|PlayMontage` (`Character.Mesh` (`self.PlayerChar`)) "/Game/MultiplayerShooter/Player/Characters/Mannequins/Animations/Manny/AM_Equip_Rifle_Standing.AM_Equip_Rifle_Standing")
    (:`OnCompleted`
      (set `self.StateChar` "NewEnumerator0"))
    (:`OnNotifyBegin`
      (if (== _notifyname "ChangeWeapon")
        (`self.Update Info Weapon`)))))

(event `Reload`
  (bind (_cachedataammocurrentweapon_currentinmagazineammo _cachedataammocurrentweapon_countammofitinmagazine _cachedataammocurrentweapon_inselfammo) (break `/Game/MultiplayerShooter/Player/Blueprints/Components/WeaponSystem/Data/S_Ammo` (`self.CacheDataAmmoCurrentWeapon`)))
  ;[0.01042 0.01042 0.01042] Reload
  (set `self.CacheDataAmmoCurrentWeapon` (`BlueprintMapLibrary.Map_Find` (`self.Ammo`) (`self.CurrentTypeWeapon`)))
  (if (> _cachedataammocurrentweapon_inselfammo 0)
    (if (!= _cachedataammocurrentweapon_currentinmagazineammo _cachedataammocurrentweapon_countammofitinmagazine)
      (set `self.StateChar` "NewEnumerator2")
      (`self.SERVER:Reload`))))

(event `CLIENT:UpdateAmmo`
  (bind (_cachedataammocurrentweapon_currentinmagazineammo _cachedataammocurrentweapon_countammofitinmagazine _cachedataammocurrentweapon_inselfammo) (break `/Game/MultiplayerShooter/Player/Blueprints/Components/WeaponSystem/Data/S_Ammo` (`self.CacheDataAmmoCurrentWeapon`)))
  (bind (_cachedataammocurrentweapon_currentinmagazineammo_2 _cachedataammocurrentweapon_countammofitinmagazine_2) (break `/Game/MultiplayerShooter/Player/Blueprints/Components/WeaponSystem/Data/S_Ammo` (`self.CacheDataAmmoCurrentWeapon`)))
  (bind _returnvalue (- _cachedataammocurrentweapon_countammofitinmagazine _cachedataammocurrentweapon_currentinmagazineammo))
  ;[0.01042 0.01042 0.01042] Reload
  (if (>= _returnvalue _cachedataammocurrentweapon_inselfammo)
    (bind _structout (setmembers `/Game/MultiplayerShooter/Player/Blueprints/Components/WeaponSystem/Data/S_Ammo` :`StructRef` (`self.CacheDataAmmoCurrentWeapon`) :`CurrentInMagazineAmmo` (+ _cachedataammocurrentweapon_currentinmagazineammo _cachedataammocurrentweapon_inselfammo) :`InSelfAmmo` 0))
    (`BlueprintMapLibrary.Map_Add` (`self.Ammo`) (`self.CurrentTypeWeapon`) _structout)
    (else
      (bind _structout_2 (setmembers `/Game/MultiplayerShooter/Player/Blueprints/Components/WeaponSystem/Data/S_Ammo` :`StructRef` (`self.CacheDataAmmoCurrentWeapon`) :`CurrentInMagazineAmmo` _cachedataammocurrentweapon_countammofitinmagazine_2 :`InSelfAmmo` (- _cachedataammocurrentweapon_inselfammo _returnvalue)))
      (`BlueprintMapLibrary.Map_Add` (`self.Ammo`) (`self.CurrentTypeWeapon`) _structout_2)))
  (`self.UpdateAmmoWidget`)
  (set `self.StateChar` "NewEnumerator0"))

(event `SERVER:Reload`
  ;[0.01042 0.01042 0.01042] Reload
  (`self.MULTICAST:Reload`))

(event `MULTICAST:Reload`
  ;[0.01042 0.01042 0.01042] Reload
  (`|PlayMontage` (`Character.Mesh` (`self.PlayerChar`)) "/Game/MultiplayerShooter/Player/Characters/Mannequins/Animations/Manny/AM_Reload_Rifle_Hip.AM_Reload_Rifle_Hip"
    (:`OnCompleted`
      (`self.CLIENT:UpdateAmmo`))))

(fn `CalculateRecoilController`
  (locals (L_CacheCurrentTimeRecoil :type "Float (double-precision)"))
  (bind _playerchar (`self.PlayerChar`))
  (`KismetSystemLibrary.K2_ClearTimer` null "StabilizationWeapon")
  (set `self.AimRotBeforShoot` (`Pawn.GetControlRotation` (`self.PlayerChar`)))
  (`Pawn.AddControllerPitchInput` _playerchar (`KismetMathLibrary.RandomFloatInRange` -0.5 -0.2))
  (`Pawn.AddControllerYawInput` _playerchar (`KismetMathLibrary.RandomFloatInRange` -0.5 0.5)))

(fn `CalculateSpawnBullet`
  (returns (BulletTransform :type "Transform Structure"))
  (locals (L_MuzzleSocLoc :type "Vector Structure") (L_BulletSpawnT :type "Transform Structure"))
  (bind _returnvalue (`SceneComponent.K2_GetComponentLocation` (`/Game/MultiplayerShooter/Player/Blueprints/BP_ThirdPersonCharacter.FollowCamera` (`self.PlayerChar`))))
  (bind _returnvalue_2 (+ _returnvalue (* (`SceneComponent.GetForwardVector` (`/Game/MultiplayerShooter/Player/Blueprints/BP_ThirdPersonCharacter.FollowCamera` (`self.PlayerChar`))) 10000.0)))
  (set `local.L_MuzzleSocLoc` (`SceneComponent.GetSocketLocation` (`/Game/MultiplayerShooter/Player/Blueprints/BP_ThirdPersonCharacter.GunStaticMesh` (`self.PlayerChar`)) "MuzzleSocket"))
  (bind (_outhit _returnvalue_3) (`KismetSystemLibrary.LineTraceSingleForObjects` _returnvalue _returnvalue_2 (`|MakeArray` "ObjectTypeQuery1" "ObjectTypeQuery2" "ObjectTypeQuery4" :!type "EObjectTypeQuery Enum")))
  (if _returnvalue_3
    (set `local.L_BulletSpawnT` (`KismetMathLibrary.MakeTransform` (`local.L_MuzzleSocLoc`) (`KismetMathLibrary.FindLookAtRotation` (`local.L_MuzzleSocLoc`) (`.ImpactPoint` (`GameplayStatics.BreakHitResult` _outhit)))))
    (else
      (set `local.L_BulletSpawnT` (`KismetMathLibrary.MakeTransform` (`local.L_MuzzleSocLoc`) (`KismetMathLibrary.FindLookAtRotation` (`local.L_MuzzleSocLoc`) _returnvalue_2)))))
  (`self.SERVER:SpawnBullet` (`local.L_BulletSpawnT`))
  (return (`local.L_BulletSpawnT`)))

(fn `Fire`
  (returns (`NoAmmo?` :type Boolean))
  (locals (L_MuzzleSocLoc :type "Vector Structure" :default (0.0 0.0 0.0)) (L_BulletSpawnT :type "Transform Structure") (L_AmmoData :type "/Game/MultiplayerShooter/Player/Blueprints/Components/WeaponSystem/Data/S_Ammo Structure"))
  (bind (_l_ammodata_currentinmagazineammo _l_ammodata_countammofitinmagazine _l_ammodata_inselfammo) (break `/Game/MultiplayerShooter/Player/Blueprints/Components/WeaponSystem/Data/S_Ammo` (`local.L_AmmoData`)))
  (bind _l_bulletspawnt_location (`KismetMathLibrary.BreakTransform` (`local.L_BulletSpawnT`)))
  (bind _output_get (set `local.L_AmmoData` (`BlueprintMapLibrary.Map_Find` (`self.Ammo`) (`self.CurrentTypeWeapon`))))
  (if (<= (`.CurrentInMagazineAmmo_14_8B29CF054E6C71855528658CC4BAA8C1` (break `/Game/MultiplayerShooter/Player/Blueprints/Components/WeaponSystem/Data/S_Ammo` _output_get)) 0)
    (`GameplayStatics.PlaySound2D` "/Game/MultiplayerShooter/Audio/Sounds/Weapons/MSS_NoAmmo.MSS_NoAmmo" 1.0 1.0 0.0 null null)
    (return true)
    (else
      (bind _bullettransform (`self.CalculateSpawnBullet`))
      (set `local.L_BulletSpawnT` _bullettransform)
      (bind _structout (setmembers `/Game/MultiplayerShooter/Player/Blueprints/Components/WeaponSystem/Data/S_Ammo` :`StructRef` (`local.L_AmmoData`) :`CurrentInMagazineAmmo` (- (`.CurrentInMagazineAmmo_14_8B29CF054E6C71855528658CC4BAA8C1` (break `/Game/MultiplayerShooter/Player/Blueprints/Components/WeaponSystem/Data/S_Ammo` (`local.L_AmmoData`))) 1)))
      (`BlueprintMapLibrary.Map_Add` (`self.Ammo`) (`self.CurrentTypeWeapon`) _structout)
      (bind _foundwidgets (`WidgetBlueprintLibrary.GetAllWidgetsOfClass` "/Game/MultiplayerShooter/Player/Widgets/WBP_PlayerHUD.WBP_PlayerHUD_C"))
      (`WCPP_PlayerHUD.UpdateAmmoWidgetComponent` (`|GetArrayItem` _foundwidgets) _l_ammodata_currentinmagazineammo _l_ammodata_inselfammo)
      (`self.SERVER:SoundShoot` _l_bulletspawnt_location)
      (return false))))

(fn `LoweringAnimRecoil`
  (bind _animbp (message `/Game/MultiplayerShooter/Player/Characters/Mannequins/Animations/BPI/BPI_AnimBP.GetMannyAnimBP` (`SkeletalMeshComponent.GetAnimInstance` (`Character.Mesh` (`self.PlayerChar`)))))
  (bind _returnvalue (`KismetMathLibrary.FInterpTo` (`/Game/MultiplayerShooter/Player/Characters/Mannequins/Animations/ABP_Manny.AlphaRecoilFire` _animbp) 0.0 (`GameplayStatics.GetWorldDeltaSeconds`) 2.0))
  (`self.SERVER:SetLoweringRecoil` _returnvalue)
  (if (`KismetMathLibrary.NearlyEqual_FloatFloat` _returnvalue 0.0 0.05)
    (`self.SERVER:SetLoweringRecoil` 0.0)
    (`self.ResetTimerLoweringRecoil`)
    (`KismetSystemLibrary.K2_ClearTimer` null "LoweringAnimRecoil")))

(fn `SetAimRot`
  (locals (L_MuzzleSocLoc :type "Vector Structure") (L_OffsetRotWeapon :type "Rotator Structure" :default (struct)))
  (bind _returnvalue (`SceneComponent.K2_GetComponentLocation` (`/Game/MultiplayerShooter/Player/Blueprints/BP_ThirdPersonCharacter.FollowCamera` (`self.PlayerChar`))))
  (bind _returnvalue_2 (+ _returnvalue (* (`SceneComponent.GetForwardVector` (`/Game/MultiplayerShooter/Player/Blueprints/BP_ThirdPersonCharacter.FollowCamera` (`self.PlayerChar`))) 10000.0)))
  (set `local.L_MuzzleSocLoc` (`SceneComponent.GetSocketLocation` (`/Game/MultiplayerShooter/Player/Blueprints/BP_ThirdPersonCharacter.GunStaticMesh` (`self.PlayerChar`)) "MuzzleSocket"))
  (bind (_outhit _returnvalue_3) (`KismetSystemLibrary.LineTraceSingleForObjects` _returnvalue _returnvalue_2 (`|MakeArray` "ObjectTypeQuery1" "ObjectTypeQuery2" "ObjectTypeQuery4" :!type "EObjectTypeQuery Enum")))
  (if _returnvalue_3
    (set `local.L_OffsetRotWeapon` (`KismetMathLibrary.NormalizedDeltaRotator` (`SceneComponent.K2_GetComponentRotation` (`/Game/MultiplayerShooter/Player/Blueprints/BP_ThirdPersonCharacter.GunStaticMesh` (`self.PlayerChar`))) (`KismetMathLibrary.FindLookAtRotation` (`local.L_MuzzleSocLoc`) (`.ImpactPoint` (`GameplayStatics.BreakHitResult` _outhit)))))
    (else
      (set `local.L_OffsetRotWeapon` (`KismetMathLibrary.NormalizedDeltaRotator` (`SceneComponent.K2_GetComponentRotation` (`/Game/MultiplayerShooter/Player/Blueprints/BP_ThirdPersonCharacter.GunStaticMesh` (`self.PlayerChar`))) (`KismetMathLibrary.FindLookAtRotation` (`local.L_MuzzleSocLoc`) _returnvalue_2))))))

(fn `SetLookInput`
  (params (IA_LookInput :type "Vector2D Structure"))
  (set `self.IA_LookInput` IA_LookInput))

(fn `StabilizationWeapon`
  (bind (_aimrotbeforshoot_roll _aimrotbeforshoot_pitch _aimrotbeforshoot_yaw) (`KismetMathLibrary.BreakRotator` (`self.AimRotBeforShoot`)))
  (bind (_aimrotbeforshoot_roll_2 _aimrotbeforshoot_pitch_2 _aimrotbeforshoot_yaw_2) (`KismetMathLibrary.BreakRotator` (`self.AimRotBeforShoot`)))
  (bind (_aimrotbeforshoot_roll_3 _aimrotbeforshoot_pitch_3 _aimrotbeforshoot_yaw_3) (`KismetMathLibrary.BreakRotator` (`self.AimRotBeforShoot`)))
  (bind (_returnvalue_roll _returnvalue_pitch _returnvalue_yaw) (`KismetMathLibrary.BreakRotator` (`Pawn.GetControlRotation` (`self.PlayerChar`))))
  (bind (_returnvalue_roll_2 _returnvalue_pitch_2 _returnvalue_yaw_2) (`KismetMathLibrary.BreakRotator` (`Pawn.GetControlRotation` (`self.PlayerChar`))))
  (bind _returnvalue_roll_3 (`KismetMathLibrary.BreakRotator` (`Pawn.GetControlRotation` (`self.PlayerChar`))))
  (bind _returnvalue_roll_4 (`KismetMathLibrary.BreakRotator` (`Pawn.GetControlRotation` (`self.PlayerChar`))))
  (bind (_returnvalue_roll_5 _returnvalue_pitch_3 _returnvalue_yaw_3) (`KismetMathLibrary.BreakRotator` (`KismetMathLibrary.RInterpTo` (`KismetMathLibrary.MakeRotator` 0.0 _returnvalue_pitch_2 _returnvalue_yaw_2) (`KismetMathLibrary.MakeRotator` 0.0 _aimrotbeforshoot_pitch_2 _aimrotbeforshoot_yaw_2) (`GameplayStatics.GetWorldDeltaSeconds`) 3.0)))
  (if (== (`self.IA_LookInput`) (0.0 0.0))
    (`Controller.SetControlRotation` (`Pawn.GetController` (`self.PlayerChar`)) (`KismetMathLibrary.MakeRotator` _returnvalue_roll_4 _returnvalue_pitch_3 _returnvalue_yaw_3))
    (if (and (`KismetMathLibrary.NearlyEqual_FloatFloat` _aimrotbeforshoot_pitch_3 _returnvalue_pitch 0.03) (`KismetMathLibrary.NearlyEqual_FloatFloat` _aimrotbeforshoot_yaw_3 _returnvalue_yaw 0.03))
      (`Controller.SetControlRotation` (`Pawn.GetController` (`self.PlayerChar`)) (`KismetMathLibrary.MakeRotator` _returnvalue_roll_3 _aimrotbeforshoot_pitch _aimrotbeforshoot_yaw))
      (`KismetSystemLibrary.K2_ClearTimer` null "StabilizationWeapon"))
    (else
      (`KismetSystemLibrary.K2_ClearTimer` null "StabilizationWeapon"))))

(fn `StartResetShoot`
  (`self.ResetShoot`)
  (if (not (`self.No Ammo?`))
    (`KismetSystemLibrary.K2_SetTimerDelegate` (`|CreateDelegate` :!event `StabilizationWeapon`) 0.016 true)))

(fn `Update Info Weapon`
  (bind _returnvalue (`|GetDataTableRow` "/Game/MultiplayerShooter/Player/Blueprints/Components/WeaponSystem/Data/DT_Weapon.DT_Weapon" (`KismetStringLibrary.Conv_StringToName` (`|GetEnumeratorNameAsString` (`self.CurrentTypeWeapon`))))
    (:`then`
      (bind _output_get (set `self.CurrentWeaponData` _returnvalue))
      (`StaticMeshComponent.SetStaticMesh` (`/Game/MultiplayerShooter/Player/Blueprints/BP_ThirdPersonCharacter.GunStaticMesh` (`self.PlayerChar`)) (break `/Game/MultiplayerShooter/Player/Blueprints/Components/WeaponSystem/Data/S_Weapon` _output_get))
      (bind _animbp (message `/Game/MultiplayerShooter/Player/Characters/Mannequins/Animations/BPI/BPI_AnimBP.GetMannyAnimBP` (`SkeletalMeshComponent.GetAnimInstance` (`Character.Mesh` (`self.PlayerChar`)))))
      (set `/Game/MultiplayerShooter/Player/Characters/Mannequins/Animations/ABP_Manny.WeaponSocLHand` (`SceneComponent.GetSocketTransform` (`/Game/MultiplayerShooter/Player/Blueprints/BP_ThirdPersonCharacter.GunStaticMesh` (`self.PlayerChar`)) "LHandSocket" "RTS_Component") _animbp)
      (set `/Game/MultiplayerShooter/Player/Characters/Mannequins/Animations/ABP_Manny.WeaponData` (`self.CurrentWeaponData`) _animbp)
      (`SceneComponent.K2_SetRelativeTransform` (`/Game/MultiplayerShooter/Player/Blueprints/BP_ThirdPersonCharacter.SceneStaticDirWeapon` (`self.PlayerChar`)) (`.RelativeTDirWeaponComp_27_3B50619D4AE8A910A0B729ADAF167496` (break `/Game/MultiplayerShooter/Player/Blueprints/Components/WeaponSystem/Data/S_Weapon` (`self.CurrentWeaponData`))) false false))))

(fn `UpdateAmmoWidget`
  (bind (_cachedataammocurrentweapon_currentinmagazineammo _cachedataammocurrentweapon_countammofitinmagazine _cachedataammocurrentweapon_inselfammo) (break `/Game/MultiplayerShooter/Player/Blueprints/Components/WeaponSystem/Data/S_Ammo` (`self.CacheDataAmmoCurrentWeapon`)))
  (set `self.CacheDataAmmoCurrentWeapon` (`BlueprintMapLibrary.Map_Find` (`self.Ammo`) (`self.CurrentTypeWeapon`)))
  (bind _foundwidgets (`WidgetBlueprintLibrary.GetAllWidgetsOfClass` "/Game/MultiplayerShooter/Player/Widgets/WBP_PlayerHUD.WBP_PlayerHUD_C"))
  (`WCPP_PlayerHUD.UpdateAmmoWidgetComponent` (`|GetArrayItem` _foundwidgets) _cachedataammocurrentweapon_currentinmagazineammo _cachedataammocurrentweapon_inselfammo))