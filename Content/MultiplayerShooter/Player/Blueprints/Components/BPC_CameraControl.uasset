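; Camera control component that smoothly zooms the player character's camera by changing its CameraBoom arm length.
; BeginPlay stores the starting arm length, and StartZoomCamera targets either the zoom length or that stored default.
; A looping timer, roughly once per frame, drives the interpolation instead of Tick.
; ZoomingCamera eases the boom toward the target with FInterpTo and clears its timer by function name when nearly there.
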(event `self.ReceiveBeginPlay`
  (`parent.ReceiveBeginPlay`)
  (set `self.StartTarget Arm Length` (`SpringArmComponent.TargetArmLength` (`/Game/MultiplayerShooter/Player/Blueprints/BP_ThirdPersonCharacter.CameraBoom` (`self.PlayerChar`)))))

(event `StartZoomCamera`
  (params (`ZoomIn?` :type Boolean))
  (if `ZoomIn?`
    (set `self.CurrentTargetArmLength` (`self.TargetArmLength`))
    (else
      (set `self.CurrentTargetArmLength` (`self.StartTarget Arm Length`))))
  (`KismetSystemLibrary.K2_SetTimerDelegate` (`|CreateDelegate` :!event `ZoomingCamera`) 0.016 true))

(fn `ZoomingCamera`
  (locals (L_TargetArmLength :type "Float (double-precision)" :default 0.0))
  (bind _output_get (set `SpringArmComponent.TargetArmLength` (`KismetMathLibrary.FInterpTo` (`SpringArmComponent.TargetArmLength` (`/Game/MultiplayerShooter/Player/Blueprints/BP_ThirdPersonCharacter.CameraBoom` (`self.PlayerChar`))) (`self.CurrentTargetArmLength`) (`GameplayStatics.GetWorldDeltaSeconds`) 5.0) (`/Game/MultiplayerShooter/Player/Blueprints/BP_ThirdPersonCharacter.CameraBoom` (`self.PlayerChar`))))
  (if (`KismetMathLibrary.NearlyEqual_FloatFloat` _output_get (`self.CurrentTargetArmLength`) 1.0)
    (`KismetSystemLibrary.K2_ClearTimer` null "ZoomingCamera")))