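; BP_HPStat is the health stat in the multiplayer shooter's stats system, extending a parent stat with death on depletion.
; After the parent applies a change, a value at or below zero makes it send a SERVERDoing message for "HP" to its outer object.
; Its Doing override sends Death to the stats component's owning character through a message interface.
; It also pushes current and max HP to the player HUD widget.
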(fn `ChangeStat`
  (params (Value :type "Float (double-precision)"))
  (`parent.ChangeStat` Value)
  (if (<= (`self.CurrentValue`) 0.0)
    (bind _statcomponent (message `/Game/MultiplayerShooter/Player/Blueprints/Components/StatsSystem/BPI_StatComponent.GetStatComponent` (`KismetSystemLibrary.GetOuterObject` self)))
    (`/Game/MultiplayerShooter/Player/Blueprints/Components/StatsSystem/BPC_StatsSystem.SERVER:Doing` _statcomponent "HP")))

(fn `Doing`
  (`parent.Doing`)
  (bind _thirdpersonchar (message `/Game/MultiplayerShooter/Player/Blueprints/BPI/BPI_PlayerChar.GetThirdPersonChar` (`ActorComponent.GetOwner` (`self.StatsComponent`))))
  (`/Game/MultiplayerShooter/Player/Blueprints/BP_ThirdPersonCharacter.Death` _thirdpersonchar))

(fn `Update Stat in Widget`
  (params (Widget :type "UserWidget Object Reference"))
  (bind _playerhudwidget (message `/Game/MultiplayerShooter/Player/Widgets/BPI_WidgetHUD.GetPlayerHUDWidget` Widget))
  (`WCPP_PlayerHUD.UpdateHPWidgetComponent` _playerhudwidget (`self.CurrentValue`) (`self.MaxValue`)))