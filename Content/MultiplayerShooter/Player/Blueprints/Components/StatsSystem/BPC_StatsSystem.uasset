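; Actor component for a multiplayer shooter that manages its owner's stats as a name-keyed map of stat objects.
; On BeginPlay it gives each stat a back-reference to itself, and a server event multicasts each stat's Doing action.
; ChangeStat applies a signed delta through the stat object.
; If the owning pawn is controlled, it then has that stat update the first WBP_PlayerHUD found.
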(event `self.ReceiveBeginPlay`
  (`parent.ReceiveBeginPlay`)
  (bind _values (`BlueprintMapLibrary.Map_Values` (`self.Stats`)))
  (for _array_element _values
    (bind _basestat (message `/Game/MultiplayerShooter/Player/Blueprints/Components/StatsSystem/BPI_Stat.GetBaseStat` _array_element))
    (set `/Game/MultiplayerShooter/Player/Blueprints/Components/StatsSystem/BP_BaseStat.StatsComponent` self _basestat)))

(event `SERVER:Doing`
  (params (NameStat :type String))
  (`self.MULTICAST:Doing` NameStat))

(event `MULTICAST:Doing`
  (params (NameStat :type String))
  (bind _basestat (message `/Game/MultiplayerShooter/Player/Blueprints/Components/StatsSystem/BPI_Stat.GetBaseStat` (`BlueprintMapLibrary.Map_Find` (`self.Stats`) NameStat)))
  (`/Game/MultiplayerShooter/Player/Blueprints/Components/StatsSystem/BP_BaseStat.Doing` _basestat))

(fn `ChangeStat`
  (params (NameStat :type "String (by ref)") (MathDoing :type "/Game/MultiplayerShooter/Player/Blueprints/Components/Data/E_TypeMathDoing Enum" :default "NewEnumerator0") (Value :type "Float (double-precision)"))
  (locals (L_StatData :type "/Game/MultiplayerShooter/Player/Blueprints/Components/Data/S_Stat Structure") (L_Value :type "Float (double-precision)") (L_BaseStat :type "/Game/MultiplayerShooter/Player/Blueprints/Components/StatsSystem/BP_BaseStat Object Reference"))
  (set `local.L_Value` (`KismetMathLibrary.Abs` Value))
  (bind _basestat (message `/Game/MultiplayerShooter/Player/Blueprints/Components/StatsSystem/BPI_Stat.GetBaseStat` (`BlueprintMapLibrary.Map_Find` (`self.Stats`) (`local.NameStat`))))
  (set `local.L_BaseStat` _basestat)
  (switch `/Game/MultiplayerShooter/Player/Blueprints/Components/Data/E_TypeMathDoing` (`local.MathDoing`)
    (:`NewEnumerator0`
      _)
    (:`NewEnumerator1`
      (set `local.L_Value` (* (`local.L_Value`) -1.0))))
  (`/Game/MultiplayerShooter/Player/Blueprints/Components/StatsSystem/BP_BaseStat.ChangeStat` (`local.L_BaseStat`) (`local.L_Value`))
  (if (`Pawn.IsControlled` (cast `Pawn` (`self.GetOwner`) :!pure true))
    (`self.UpdateStatWidget` (`local.NameStat`))))

(fn `GetStatComponent`
  (returns (StatComponent :type "/Game/MultiplayerShooter/Player/Blueprints/Components/StatsSystem/BPC_StatsSystem Object Reference"))
  (return self))

(fn `UpdateStatWidget`
  (params (NameStat :type String))
  (bind _basestat (message `/Game/MultiplayerShooter/Player/Blueprints/Components/StatsSystem/BPI_Stat.GetBaseStat` (`BlueprintMapLibrary.Map_Find` (`self.Stats`) (`local.NameStat`))))
  (bind _foundwidgets (`WidgetBlueprintLibrary.GetAllWidgetsOfClass` "/Game/MultiplayerShooter/Player/Widgets/WBP_PlayerHUD.WBP_PlayerHUD_C"))
  (`/Game/MultiplayerShooter/Player/Blueprints/Components/StatsSystem/BP_BaseStat.Update Stat in Widget` _basestat (`|GetArrayItem` _foundwidgets)))