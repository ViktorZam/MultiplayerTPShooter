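; Multiplayer shooter GameState that runs the match countdown and gathers scoreboard data.
; The server starts a looping one-second timer, apparently driving TimeTick, which decrements the clamped match time and multicasts it to the player HUD widget.
; At zero, it sends a client stop-game call through each PlayerState and clears the timer by function name.
; GetDataAllPlayers builds a name-keyed map of kills, deaths and ping from PlayerArray.
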(event `self.ReceiveBeginPlay`
  (`/Engine/EditorBlueprintResources/ActorMacros.Switch Has Authority`
    (:`Authority`
      (set `self.CurrentTimeMatch` (`self.MaxTimeMatch`))
      (`KismetSystemLibrary.K2_SetTimerDelegate` (`|CreateDelegate` :!event `TimeTick`) 1.0 true))))

(event `MULTICAST:UpdateTimeWidget`
  (params (CurrentTime :type Integer))
  (bind _foundwidgets (`WidgetBlueprintLibrary.GetAllWidgetsOfClass` "/Game/MultiplayerShooter/Player/Widgets/WBP_PlayerHUD.WBP_PlayerHUD_C"))
  (bind _output (`|GetArrayItem` _foundwidgets))
  (`/Engine/EditorBlueprintResources/StandardMacros.IsValid` _output
    (:`Is Valid`
      (`WCPP_PlayerHUD.UpdateTimeWidgetComponent` _output CurrentTime))))

(fn `GetDataAllPlayers`
  (returns (PlayerData :type "Map of String to /Game/MultiplayerShooter/Player/Blueprints/PS/Data/S_PlayerData Structure"))
  (locals (L_PlayerData :type "Map of String to /Game/MultiplayerShooter/Player/Blueprints/PS/Data/S_PlayerData Structure") (L_PS :type "/Game/MultiplayerShooter/Player/Blueprints/PS/BP_PS Object Reference") (L_NameInfo :type "Array of String") (L_CurrentValues :type "Array of Float (double-precision)"))
  (for _array_element (`self.PlayerArray`)
    (bind _ps (message `/Game/MultiplayerShooter/Player/Blueprints/BPI/BPI_PS.GetPS` _array_element))
    (set `local.L_PS` _ps)
    (for _array_element_2 (`local.L_NameInfo`)
      (bind _currentvalue (`/Game/MultiplayerShooter/Player/Blueprints/PS/BP_PS.GetDataFromPlayerInfo` (`local.L_PS`) _array_element_2))
      (`KismetArrayLibrary.Array_Add` (`local.L_CurrentValues`) _currentvalue))
    (`BlueprintMapLibrary.Map_Add` (`local.L_PlayerData`) (`/Game/MultiplayerShooter/Player/Blueprints/PS/BP_PS.PlayerNameInGame` (`local.L_PS`)) (make `/Game/MultiplayerShooter/Player/Blueprints/PS/Data/S_PlayerData` (`KismetMathLibrary.FTrunc` (`|GetArrayItem` (`local.L_CurrentValues`))) (`KismetMathLibrary.FTrunc` (`|GetArrayItem` (`local.L_CurrentValues`) 1)) (`KismetMathLibrary.FTrunc` (`PlayerState.GetPingInMilliseconds` (`local.L_PS`)))))
    (`KismetArrayLibrary.Array_Clear` (`local.L_CurrentValues`)))
  (return (`local.L_PlayerData`)))

(fn `GetGS`
  (returns (GS :type "/Game/MultiplayerShooter/Player/Blueprints/BP_GS Object Reference"))
  (return self))

(fn `TimeTick`
  (bind _output_get (set `self.CurrentTimeMatch` (`KismetMathLibrary.Clamp` (- (`self.CurrentTimeMatch`) 1) 0 (`self.MaxTimeMatch`))))
  (`self.MULTICAST:UpdateTimeWidget` _output_get)
  (if (== (`self.CurrentTimeMatch`) 0)
    (for _array_element (`self.PlayerArray`)
      (bind _ps (message `/Game/MultiplayerShooter/Player/Blueprints/BPI/BPI_PS.GetPS` _array_element))
      (`/Game/MultiplayerShooter/Player/Blueprints/PS/BP_PS.CLIENT:StopGame` _ps true))
    (`KismetSystemLibrary.K2_ClearTimer` null "TimeTick")))

(fn `UserConstructionScript`)